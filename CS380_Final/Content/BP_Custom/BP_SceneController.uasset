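; BP_SceneController sets up a driving scene when play begins.
; It blends player 0's view to ViewCam, then spawns a SportsCar_Pawn and a separate VehiclePlayerController at StartLine.
; It creates a VehicleUI in MPH mode owned by the new controller, then hands that controller the car's movement component and the HUD.
; No possession or add-to-viewport call happens in this Blueprint.
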(event `self.ReceiveBeginPlay`
  (bind _returnvalue (`KismetMathLibrary.Conv_VectorToTransform` (`self.StartLine`)))
  (`PlayerController.SetViewTargetWithBlend` (`GameplayStatics.GetPlayerController` 0) (`self.ViewCam`) 0.0 "VTBlend_Linear" 0.0 false)
  (bind _returnvalue_2 (`|SpawnActorFromClass` "/Game/VehicleTemplate/Blueprints/SportsCar/SportsCar_Pawn.SportsCar_Pawn_C" _returnvalue "AlwaysSpawn" "OverrideRootScale" null null))
  (bind _returnvalue_3 (`|SpawnActorFromClass` "/Game/VehicleTemplate/Blueprints/VehiclePlayerController.VehiclePlayerController_C" _returnvalue "Undefined" "OverrideRootScale" null null))
  (bind _returnvalue_4 (`|CreateWidget` "/Game/VehicleTemplate/Blueprints/VehicleUI.VehicleUI_C" _returnvalue_3 true))
  (set `/Game/VehicleTemplate/Blueprints/VehiclePlayerController.Vehicle Movement Component` (`WheeledVehiclePawn.VehicleMovementComponent` _returnvalue_2) _returnvalue_3)
  (set `/Game/VehicleTemplate/Blueprints/VehiclePlayerController.VehicleHud` _returnvalue_4 _returnvalue_3))

(fn `UserConstructionScript`)