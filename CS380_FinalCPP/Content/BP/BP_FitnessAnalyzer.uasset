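; BP_FitnessAnalyzer tracks a marble's run for fitness scoring, counting time, checkpoints hit and off-track penalties.
; Each Tick adds to elapsed time, flags the marble for destruction at its time limit, and otherwise accumulates a per-frame off-track punishment.
; CalcFitness only returns the stored Fitness, which nothing here computes; data gathering, center-distance and time-update functions are empty stubs.
; BeginPlay forces the marble's debug flag on, printing elapsed time every frame.
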(event `self.ReceiveBeginPlay`
  (set `/Game/BP/SceneActors/BP_Marble.Debug` true (`self.Marble`)))

(event `self.ReceiveTick`
  (params (DeltaSeconds :type "Float (single-precision)"))
  (bind _marble (`self.Marble`))
  (`self.DebugPrint`)
  (bind _output_get (set `self.CurrTime` (+ DeltaSeconds (`self.CurrTime`))))
  (if (>= _output_get (`/Game/BP/SceneActors/BP_Marble.TimeLimit` _marble))
    (`self.MarkDestroy`)
    (elif (not (`/Game/BP/SceneActors/BP_Marble.IsOnTrack` _marble))
      (set `self.OffTrack_Fitness` (+ (`self.OffTrack_Fitness`) (`self.OffTrack_Punishment`))))))

(event `GatherData`)

(fn `AggregateDistanceFromCenter`
  (params (Marble :type "/Game/BP/SceneActors/BP_Marble Object Reference")))

(fn `Calc_Fitness`
  (returns (Fitness :type "Float (double-precision)"))
  (return (`self.Fitness`)))

(fn `DebugPrint`
  (if (`/Game/BP/SceneActors/BP_Marble.Debug` (`self.Marble`))
    (`KismetSystemLibrary.PrintString` (`KismetStringLibrary.Conv_DoubleToString` (`self.CurrTime`)))))

(fn `IncrementCheckpoint`
  (`/Engine/EditorBlueprintResources/StandardMacros.IncrementInt` (`self.CheckpointsHit`)))

(fn `MarkDestroy`
  (set `/Game/BP/SceneActors/BP_Marble.Destroy` true (`self.Marble`)))

(fn `UpdateTime`
  (params (DT :type "Float (double-precision)")))