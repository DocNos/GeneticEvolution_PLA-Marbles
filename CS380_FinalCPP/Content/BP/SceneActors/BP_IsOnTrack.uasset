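; BP_IsOnTrack measures how a Sphere tracks against the BP_SplineActor spline.
; Each tick it adds the distance to the closest spline point to a printed running total.
; It also stores a normalized left or right angle from the acos of both world position vectors, which is never negative.
; A short debug-drawn trace along world +Y records wall distance when it hits a BP_Wall.
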(event `self.ReceiveBeginPlay`
  (bind _returnvalue (`GameplayStatics.GetActorOfClass` "/Game/BP/SceneActors/BP_SplineActor.BP_SplineActor_C"))
  (set `self.SplineRef` _returnvalue))

(event `self.ReceiveTick`
  (params (DeltaSeconds :type "Float (single-precision)"))
  (bind _returnvalue (`KismetMathLibrary.TransformLocation` (`SceneComponent.K2_GetComponentToWorld` (`Actor.RootComponent` (`self.Sphere`)))))
  (bind _returnvalue_2 (`SplineComponent.FindLocationClosestToWorldLocation` (`/Game/BP/SceneActors/BP_SplineActor.Spline` (`self.SplineRef`)) _returnvalue "World"))
  (bind _returnvalue_3 (`KismetMathLibrary.Vector_Distance` _returnvalue _returnvalue_2))
  (bind _returnvalue_4 (`KismetMathLibrary.DegAcos` (/ (`KismetMathLibrary.Dot_VectorVector` _returnvalue _returnvalue_2) (* (`KismetMathLibrary.VSize` _returnvalue) (`KismetMathLibrary.VSize` _returnvalue_2)))))
  (if (<= _returnvalue_3 0.0)
    (bind _output_get (set `self.TotalAbsoluteDistFromCenter` (+ (* _returnvalue_3 -1.0) (`self.TotalAbsoluteDistFromCenter`))))
    (`KismetSystemLibrary.PrintString` (`KismetStringLibrary.Conv_DoubleToString` _output_get))
    (else
      (bind _output_get_2 (set `self.TotalAbsoluteDistFromCenter` (+ _returnvalue_3 (`self.TotalAbsoluteDistFromCenter`))))
      (`KismetSystemLibrary.PrintString` (`KismetStringLibrary.Conv_DoubleToString` _output_get_2) true true (struct :`R` 0.2097 :`G` 1.0 :`A` 1.0) 0.0)))
  (if (> _returnvalue_4 0.0)
    (set `self.AngleFromSplineRight` (`KismetMathLibrary.NormalizeToRange` _returnvalue_4 0.0 360.0))
    (set `self.AngleFromSplineLeft` 0.0)
    (else
      (set `self.AngleFromSplineLeft` (`KismetMathLibrary.NormalizeToRange` _returnvalue_4 -360.0))
      (set `self.AngleFromSplineRight` 0.0)))
  (bind _outhit (`KismetSystemLibrary.LineTraceSingle` :`Start` _returnvalue :`End` (+ _returnvalue (0.0 100.0 0.0)) :`TraceChannel` "TraceTypeQuery1" :`DrawDebugType` "ForOneFrame"))
  (bind (_bblockinghit _binitialoverlap _time _distance _location _impactpoint _normal _impactnormal _physmat _hitactor) (`GameplayStatics.BreakHitResult` _outhit))
  (cast `/Game/BP/SceneActors/BP_Wall` _hitactor)
  (set `self.DistFromNearestWall` _distance))