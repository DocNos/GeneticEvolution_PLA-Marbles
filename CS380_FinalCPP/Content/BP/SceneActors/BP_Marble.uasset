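; BP_Marble is a physics-driven marble actor that hands references to fitness-analyzer and on-track components at construction.
; Helper functions accumulate forward, right and up vectors, which Tick applies to the sphere as one impulse, then clears.
; CheckIfOnTrack, not called here, totals distance from the closest BP_SplineActor spline point and compares it to track half-width.
; As written, that check sets IsOnTrack true only when distance exactly equals half-width.
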(event `self.ReceiveBeginPlay`
  (bind _returnvalue (`GameplayStatics.GetActorOfClass` "/Game/BP/SceneActors/BP_SplineActor.BP_SplineActor_C"))
  (set `self.SplineRef` _returnvalue)
  (set `self.IsOnTrack` true))

(event `self.ReceiveTick`
  (params (DeltaSeconds :type "Float (single-precision)"))
  (`self.DebugPrint`)
  (set `self.CurrSpeed` (`KismetMathLibrary.VSize` (`SceneComponent.GetComponentVelocity` (`self.Sphere`))))
  (`self.AddVelocity`))

(fn `AddForwardVelocity`
  (params (Positive :type Boolean))
  (bind _forwardvel (`self.ForwardVel`))
  (if Positive
    (set `self.ForwardVel` (+ (* (`self.ForwardAccScale`) (`self.ForwardDir`)) _forwardvel))
    (else
      (set `self.ForwardVel` (+ _forwardvel (* (* (`self.ForwardAccScale`) -1.0) (`self.ForwardDir`)))))))

(fn `AddRightVelocity`
  (params (Positive :type Boolean))
  (bind _rightvel (`self.RightVel`))
  (if Positive
    (set `self.RightVel` (+ (* (`self.RightAccScale`) (`self.RightDir`)) _rightvel))
    (else
      (set `self.RightVel` (+ _rightvel (* (* (`self.RightAccScale`) -1.0) (`self.RightDir`)))))))

(fn `AddUpVelocity`
  (set `self.UpVel` (+ (`self.UpVel`) (* (`self.UpDir`) (`self.UpAccScale`)))))

(fn `AddVelocity`
  (bind _returnvalue (+ (`self.ForwardVel`) (`self.RightVel`) (`self.UpVel`)))
  (if (> (`KismetMathLibrary.VSize` _returnvalue) 0.0)
    (`PrimitiveComponent.AddImpulse` (`self.Sphere`) _returnvalue "None" false)
    (set `self.ForwardVel` (0.0 0.0 0.0))
    (set `self.RightVel` (0.0 0.0 0.0))
    (set `self.UpVel` (0.0 0.0 0.0))))

(fn `CheckIfOnTrack`
  (bind _trackhalfwidth (`self.TrackHalfWidth`))
  (bind _returnvalue (`KismetMathLibrary.TransformLocation` (`SceneComponent.K2_GetComponentToWorld` (`self.Sphere`))))
  (bind _returnvalue_2 (`KismetMathLibrary.Vector_Distance` _returnvalue (`SplineComponent.FindLocationClosestToWorldLocation` (`/Game/BP/SceneActors/BP_SplineActor.Spline` (`self.SplineRef`)) _returnvalue "World")))
  (bind _returnvalue_3 (> _returnvalue_2 _trackhalfwidth))
  (bind _returnvalue_4 (< _returnvalue_2 _trackhalfwidth))
  (if (<= _returnvalue_2 0.0)
    (set `self.TotalAbsoluteDistFromCenter` (+ (* _returnvalue_2 -1.0) (`self.TotalAbsoluteDistFromCenter`)))
    (else
      (set `self.TotalAbsoluteDistFromCenter` (+ _returnvalue_2 (`self.TotalAbsoluteDistFromCenter`)))))
  (bind _output_get (set `self.IsOnTrack` (not (or _returnvalue_3 _returnvalue_4))))
  (if (and (not _output_get) (`self.Debug`))
    (`KismetSystemLibrary.PrintString` (`KismetStringLibrary.Conv_BoolToString` _output_get) true true (struct :`G` 0.66 :`B` 1.0 :`A` 1.0) 0.0))
  (set `self.MovingLeft` _returnvalue_3)
  (set `self.MovingRight` _returnvalue_4))

(fn `DebugPrint`
  (if (`self.Debug`)
    (`KismetSystemLibrary.PrintString` (`KismetStringLibrary.Concat_StrStr` (`self.Identifier`) " Speed: " (`KismetSystemLibrary.MakeLiteralString` (`KismetStringLibrary.Conv_DoubleToString` (`KismetMathLibrary.VSize` (`SceneComponent.GetComponentVelocity` (`self.Sphere`)))))) true true (struct :`G` 0.66 :`B` 1.0 :`A` 1.0) 0.0)))

(fn `KillVelocity`
  (set `self.RightVel` (* (`self.RightVel`) -1.0))
  (set `self.ForwardVel` (* (`self.ForwardVel`) -1.0))
  (set `self.UpVel` (* (`self.UpVel`) -1.0)))

(fn `SetVelocity`
  (params (Velocity :type "Vector Structure"))
  (bind (_x _y _z) (`KismetMathLibrary.BreakVector3f` Velocity))
  (set `self.RightVel` (`KismetMathLibrary.MakeVector` (+ (.x (+ (`self.ForwardVel`) (`self.ForwardVel`) (`self.UpVel`))) _x)))
  (set `self.ForwardVel` (`KismetMathLibrary.MakeVector` 0.0 (+ (.y (+ (`self.ForwardVel`) (`self.ForwardVel`) (`self.UpVel`))) _y)))
  (set `self.UpVel` (`KismetMathLibrary.MakeVector` 0.0 0.0 (+ (.z (+ (`self.ForwardVel`) (`self.ForwardVel`) (`self.UpVel`))) _z))))

(fn `UserConstructionScript`
  (set `/Game/BP/BP_FitnessAnalyzer.Marble` self (`self.BP_FitnessAnalyzer`))
  (set `/Game/BP/SceneActors/BP_IsOnTrack.Sphere` self (`self.BP_IsOnTrack`)))