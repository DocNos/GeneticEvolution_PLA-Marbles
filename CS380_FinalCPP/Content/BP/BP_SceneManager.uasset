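; BP_SceneManager sets up a genetic algorithm simulation scene, including its camera and UI.
; The construction script passes the AI controller to GeneticAlgorithm, creates the initial generation and resets the generation counter.
; Gene count follows enum entry counts, layer count and layer width, matching the weight count of a fully connected neural network.
; BeginPlay switches the player's view to SceneCam and shows WB_SimUI with a reference back to the manager.
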(event `self.ReceiveBeginPlay`
  (`PlayerController.SetViewTargetWithBlend` (`GameplayStatics.GetPlayerController` 0) (`self.SceneCam`) 0.0 "VTBlend_Linear" 0.0 false)
  (bind _returnvalue (`|CreateWidget` "/Game/BP/Widgets/WB_SImUI.WB_SimUI_C"))
  (`UserWidget.AddToViewport` _returnvalue 0)
  (set `/Game/BP/Widgets/WB_SImUI.SceneManager` self _returnvalue))

(fn `UserConstructionScript`
  (bind _geneticalgorithm (`self.GeneticAlgorithm`))
  (bind _geneticalgorithm_2 (`self.GeneticAlgorithm`))
  (bind _numperlayer (`/Game/BP/AIControl/GeneticAlgorithm.numPerLayer` _geneticalgorithm_2))
  (set `/Game/BP/AIControl/GeneticAlgorithm.AIcontroller` (`self.AIController`) _geneticalgorithm)
  (set `/Game/BP/AIControl/GeneticAlgorithm.geneNumber` (+ (* (enumcount `ESensoryType`) _numperlayer) (* (- (`/Game/BP/AIControl/GeneticAlgorithm.numLayers` _geneticalgorithm_2) 1) _numperlayer _numperlayer) (* (enumcount `EActionType`) _numperlayer)) _geneticalgorithm)
  (`/Game/BP/AIControl/GeneticAlgorithm.CreateInitialGeneration` _geneticalgorithm)
  (set `/Game/BP/AIControl/GeneticAlgorithm.Generation Number` 0 _geneticalgorithm))